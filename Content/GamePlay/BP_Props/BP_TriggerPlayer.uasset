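; BP_TriggerPlayer is a prop actor that reacts to other actors overlapping it, currently only as a debug trigger.
; Begin and end overlap events forward the other actor to OnActorTriggerEnter and OnActorTriggerLeave functions.
; Each function prints a fixed tag plus that actor's display name in its own color, with no filtering for the player.
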(event `self.ReceiveActorBeginOverlap`
  (params (OtherActor :type "Actor Object Reference"))
  (`self.OnActorTriggerEnter` OtherActor))

(event `self.ReceiveActorEndOverlap`
  (params (OtherActor :type "Actor Object Reference"))
  (`self.OnActorTriggerLeave` OtherActor))

(fn `OnActorTriggerEnter`
  (params (Actor :type "Actor Object Reference"))
  (`KismetSystemLibrary.PrintString` (`KismetStringLibrary.Concat_StrStr` "ChuiDedan" (`KismetSystemLibrary.GetDisplayName` Actor)) true true (struct :`R` 0.872257 :`B` 1.0 :`A` 1.0)))

(fn `OnActorTriggerLeave`
  (params (Actor :type "Actor Object Reference"))
  (`KismetSystemLibrary.PrintString` (`KismetStringLibrary.Concat_StrStr` "ChuiPoDan" (`KismetSystemLibrary.GetDisplayName` Actor)) true true (struct :`R` 1.0 :`B` 0.682308 :`A` 1.0)))

(fn `UserConstructionScript`)