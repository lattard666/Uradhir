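; BP_Trampoline is a prop that launches the player when they enter its trigger.
; It extends a parent trigger class, running the parent's enter handler before calling Jump.
; Jump launches the PlayerTrigger character along the Box component's forward vector scaled by PowerJump, adding to existing velocity instead of overriding it.
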(event `self.ReceiveTick`
  (params (DeltaSeconds :type "Float (single-precision)")))

(fn `jump`
  (`Character.LaunchCharacter` (`self.PlayerTrigger`) (* (`self.PowerJump`) (`SceneComponent.GetForwardVector` (`self.Box`))) false false))

(fn `OnActorTriggerEnter`
  (params (Actor :type "Actor Object Reference"))
  (`parent.OnActorTriggerEnter` Actor)
  (`self.jump`))

(fn `UserConstructionScript`
  (`parent.UserConstructionScript`))