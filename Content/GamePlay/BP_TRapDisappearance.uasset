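; BP_TRapDisappearance is a single-use trap that damages the player and then disappears.
; It extends a parent trigger class, calling the parent's OnActorTriggerEnter before running its own Dommage function.
; Dommage subtracts Degat from LifeCurrent on PlayerTrigger, which this Blueprint never sets itself, then destroys the trap actor.
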(event `self.ReceiveTick`
  (params (DeltaSeconds :type "Float (single-precision)")))

(fn `Dommage`
  (bind _playertrigger (`self.PlayerTrigger`))
  (set `/Game/ThirdPerson/Blueprints/BP_ThirdPersonCharacter.Life_Current` (- (`/Game/ThirdPerson/Blueprints/BP_ThirdPersonCharacter.Life_Current` _playertrigger) (`self.Degat`)) _playertrigger)
  (`self.K2_DestroyActor`))

(fn `OnActorTriggerEnter`
  (params (Actor :type "Actor Object Reference"))
  (`parent.OnActorTriggerEnter` Actor)
  (`self.Dommage`))

(fn `UserConstructionScript`
  (`parent.UserConstructionScript`))