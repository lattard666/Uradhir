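; Base trigger Blueprint that tracks when the player character is inside it.
; On trigger enter, it calls the parent handler, then casts the actor to BP_ThirdPersonCharacter and stores it in PlayerTrigger.
; On trigger leave, it calls the parent handler and clears PlayerTrigger if the leaving actor matches the stored one.
; The event graph and construction script add no logic of their own.
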(event `self.K2_OnBecomeViewTarget`
  (params (PC :type "PlayerController Object Reference")))

(fn `OnActorTriggerEnter`
  (params (Actor :type "Actor Object Reference"))
  (`parent.OnActorTriggerEnter` Actor)
  (bind _asbp_third_person_character (cast `/Game/ThirdPerson/Blueprints/BP_ThirdPersonCharacter` Actor))
  (set `self.PlayerTrigger` _asbp_third_person_character))

(fn `OnActorTriggerLeave`
  (params (Actor :type "Actor Object Reference"))
  (`parent.OnActorTriggerLeave` Actor)
  (if (== Actor (`self.PlayerTrigger`))
    (set `self.PlayerTrigger` null)))

(fn `UserConstructionScript`
  (`parent.UserConstructionScript`))