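; Trigger actor that returns the player to the last saved checkpoint when its parent's actor-enter event fires, loading saved state rather than writing it.
; BeginPlay caches player 0's BP_ThirdPersonCharacter, and the overridden OnActorTriggerEnter calls Checkpoint after the parent logic, without checking which actor entered.
; Checkpoint loads BP_SAveGame from the "Game" slot if it exists, restores the player's life and teleports them to the saved location.
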(event `self.ReceiveBeginPlay`
  (bind _asbp_third_person_character (cast `/Game/ThirdPerson/Blueprints/BP_ThirdPersonCharacter` (`GameplayStatics.GetPlayerCharacter` 0)))
  (set `self.Player` _asbp_third_person_character))

(fn `Checkpoint`
  (bind _returnvalue (`GameplayStatics.DoesSaveGameExist` "Game"))
  (if _returnvalue
    (bind _returnvalue_2 (`GameplayStatics.LoadGameFromSlot` "Game"))
    (bind _asbp_save_game (cast `/Game/GamePlay/BP_Gampeplay/BP_SAveGame` _returnvalue_2))
    (set `/Game/ThirdPerson/Blueprints/BP_ThirdPersonCharacter.Life_Current` (`/Game/GamePlay/BP_Gampeplay/BP_SAveGame.Life` _asbp_save_game) (`self.Player`))
    (`self.K2_SetActorLocation` (`self.Player`) (`/Game/GamePlay/BP_Gampeplay/BP_SAveGame.Location` _asbp_save_game) false true)))

(fn `OnActorTriggerEnter`
  (params (Actor :type "Actor Object Reference"))
  (`parent.OnActorTriggerEnter` Actor)
  (`self.Checkpoint`))

(fn `UserConstructionScript`
  (`parent.UserConstructionScript`))