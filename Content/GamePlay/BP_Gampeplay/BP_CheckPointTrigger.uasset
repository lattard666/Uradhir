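; BP_CheckPointTrigger is a checkpoint trigger that saves the player's position when an actor enters it.
; It caches the first-person character at BeginPlay and overrides the parent's trigger-enter hook to call Checkpoint, without checking which actor entered.
; Checkpoint writes the player's location into a new BP_SAveGame and saves it to the "Game" slot.
; Life is not saved: LifeCurrent is assigned to itself and the Life write is disconnected.
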(event `self.ReceiveBeginPlay`
  (bind _asbp_first_person_character (cast `/Game/FirstPerson/Blueprints/BP_FirstPersonCharacter` (`GameplayStatics.GetPlayerCharacter` 0)))
  (set `self.Player` _asbp_first_person_character))

(fn `Checkpoint`
  (bind _player (`self.Player`))
  (bind _returnvalue (`GameplayStatics.CreateSaveGameObject` "/Game/GamePlay/BP_Gampeplay/BP_SAveGame.BP_SAveGame_C"))
  (set `/Game/FirstPerson/Blueprints/BP_FirstPersonCharacter.Life_Current` (`/Game/FirstPerson/Blueprints/BP_FirstPersonCharacter.Life_Current` _player) _player)
  (set `/Game/GamePlay/BP_Gampeplay/BP_SAveGame.Location` (`self.K2_GetActorLocation` (`self.Player`)) _returnvalue)
  (`GameplayStatics.SaveGameToSlot` _returnvalue "Game"))

(fn `OnActorTriggerEnter`
  (params (Actor :type "Actor Object Reference"))
  (`parent.OnActorTriggerEnter` Actor)
  (`self.Checkpoint`))

(fn `UserConstructionScript`
  (`parent.UserConstructionScript`))